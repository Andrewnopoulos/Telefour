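; Example actor that plays a team-colored translocator departure effect on a skeletal body after a timed delay.
; Burst aims at the target destination, or a fixed X offset if none, then fires flash and streak particles.
; That direction also drives a dynamic distortion material on the body, whose opacity and displacement follow a fade timeline before the body is hidden.
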(event `self.ReceiveBeginPlay`
  (`KismetSystemLibrary.K2_SetTimer` null "Burst" (`self.Delay`)))

(event `Burst`
  (bind _body (`self.Body`))
  (bind _fadeshader (`self.FadeShader`))
  (bind _firstflash (`self.FirstFlash`))
  (bind _streak (`self.Streak`))
  (bind _fadeshader_2 (`self.FadeShader`))
  (bind _targetdestination (`self.TargetDestination`))
  (bind _returnvalue (`SceneComponent.K2_GetComponentLocation` (`self.Streak`)))
  ;[1 1 1] Team Color setup for body shader
  (`MaterialInstanceDynamic.SetVectorParameterValue` (`self.FadeShader`) "TeamColor" (`self.Team Color`))
  ;[0.5652 0.4203 1] Orientation used throughout for direction effect
  (set `self.Orientation` (`KismetMathLibrary.FindLookAtRotation` _returnvalue (`KismetMathLibrary.SelectVector` (- _returnvalue (500.0 0.0 0.0)) (`self.K2_GetActorLocation` _targetdestination) (== _targetdestination null))))
  ;[1 1 1] Set teamcolor and activate first particle effect
  (`ParticleSystemComponent.SetVectorParameter` _firstflash "TeamColor" (`KismetMathLibrary.Conv_LinearColorToVector` (`self.Team Color`)))
  (`ActorComponent.Activate` _firstflash false)
  ;[1 0.1347 0.6206] Setup shader on SkelMesh
  ;;[1 0.3706 0.1875] Passes in orientation as a vector for distortion shader on body
  (`MaterialInstanceDynamic.SetVectorParameterValue` (`self.FadeShader`) "Direction" (`KismetMathLibrary.Conv_VectorToLinearColor` (`KismetMathLibrary.GreaterGreater_VectorRotator` (1.0 0.0 0.0) (`self.Orientation`))))
  (`PrimitiveComponent.SetMaterial` _body 0 _fadeshader_2)
  (`PrimitiveComponent.SetMaterial` _body 1 _fadeshader_2)
  (`PrimitiveComponent.SetMaterial` _body 2 _fadeshader_2)
  ;[0.5314 1 0.608] Set SkelMesh parameter value and orientation (derived earlier) for second particle effect
  (`ParticleSystemComponent.SetActorParameter` _streak "Player" self)
  (`SceneComponent.K2_SetWorldRotation` _streak (`self.Orientation`) false)
  ;[0.6959 1 0.7651] Set color for second particle effect and activate
  (`ParticleSystemComponent.SetVectorParameter` _streak "TeamColor" (`KismetMathLibrary.Conv_LinearColorToVector` (`self.Team Color`)))
  (`ActorComponent.Activate` _streak true)
  ;[1 0.7345 0.4852] Execute TransFadeCurve over .3 seconds
  (bind (_direction _translocatefade_curve) (`Timeline|Fade` :!via `PlayFromStart`)
    (:`Update`
      ;[0.55 0.55 0.55] Fade Opacity scalar param for Body shader
      (`MaterialInstanceDynamic.SetScalarParameterValue` _fadeshader "Opacity" _translocatefade_curve)
      ;[1 0.2413 0.1552] Lerp Displace Amount scalar param for Body shader
      (`MaterialInstanceDynamic.SetScalarParameterValue` _fadeshader "Displace Amount" (`KismetMathLibrary.Lerp` 80.0 1.0 _translocatefade_curve)))
    (:`Finished`
      (`SceneComponent.SetHiddenInGame` (`self.Body`) true true))))

(event `self.ReceiveActorBeginOverlap`
  (params (OtherActor :type "Actor Object Reference")))

(event `self.ReceiveTick`
  (params (DeltaSeconds :type "Float (single-precision)")))

(fn `UserConstructionScript`
  (bind _returnvalue (`PrimitiveComponent.CreateDynamicMaterialInstance` (`self.Body`) 4 "/Game/RestrictedAssets/Weapons/Translocator/Mat/M_Translocate_Surface_Red.M_Translocate_Surface_Red"))
  (set `self.FadeShader` _returnvalue))